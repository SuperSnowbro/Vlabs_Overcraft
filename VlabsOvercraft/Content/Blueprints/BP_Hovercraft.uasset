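; BP_Hovercraft is a drivable hovercraft moved by physics forces on its Cube component.
; A HoverPush event applies a supplied force at a given hover component's location, so lift can act at separate points on the body.
; MoveForward input pushes along the Cube's right vector, scaled by Speed.
; Turn input adds mass-independent yaw torque, scaled by TurnRate.
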(event `/Game/Blueprints/BPI_HoverVehicle.ReceiveHoverPush`
  (params (Push :type "Vector Structure") (HoverComp :type "/Game/Blueprints/BP_HoverComponent Object Reference"))
  (`PrimitiveComponent.AddForceAtLocation` (`self.Cube`) Push (`SceneComponent.K2_GetComponentLocation` HoverComp) "None"))

(event `InputAxis|MoveForward`
  (params (AxisValue :type "Float (single-precision)"))
  (`PrimitiveComponent.AddForce` (`self.Cube`) (* (`SceneComponent.GetRightVector` (`self.Cube`)) (* AxisValue (`self.Speed`))) "None" false))

(event `InputAxis|Turn`
  (params (AxisValue :type "Float (single-precision)"))
  (`PrimitiveComponent.AddTorque` (`self.Cube`) (`KismetMathLibrary.MakeVector` 0.0 0.0 (* AxisValue (`self.TurnRate`))) "None" true))

(fn `UserConstructionScript`)